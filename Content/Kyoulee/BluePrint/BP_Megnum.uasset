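; BP_Megnum is a grabbable VR magnum revolver that plays a fire sound when shot.
; Grab events toggle input and the per-hand weapon mapping context, though dropping leaves IsGrab true.
; Shoot actions call FireGun only for the holding hand.
; A six-bullet array is filled on BeginPlay, but LoadBullet is never called and HammerReload, which rotates hammer and cylinder and advances BulletIndex, is disconnected.
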(event `self.ReceiveBeginPlay`
  (`self.SettingBulletArray`)
  (set `self.BulletIndex` 0))

(event `self.ReceiveTick`
  (params (DeltaSeconds :type "Float (single-precision)")))

(event `HammerSet`
  (bind (_returnvalue_roll _returnvalue_pitch) (`KismetMathLibrary.BreakRotator` (`SceneComponent.GetSocketRotation` (`self.Hammer`) "None")))
  ;[1 1 1] 필요시 if문 추가할것
  (set `self.HammerReloading` (< _returnvalue_pitch 50.0)))

(event `FireGun`
  (`GameplayStatics.PlaySoundAtLocation` (`self.FireSound`) (`self.K2_GetActorLocation`) (struct) 1.0 1.0 0.0 null null null null))

(event `EnhancedInput|/Game/VRTemplate/Input/Actions/IA_Menu_Cursor_Right`
  (params (ActionValue :type "Vector2D Structure") (ElapsedSeconds :type "Float (double-precision)") (TriggeredSeconds :type "Float (double-precision)") (InputAction :type "InputAction Object Reference" :default "/Game/VRTemplate/Input/Actions/IA_Menu_Cursor_Right.IA_Menu_Cursor_Right"))
  (:`Triggered`
    (`KismetSystemLibrary.PrintString` "Hello")))

(event `EnhancedInput|/Game/VRTemplate/Input/Actions/IA_Shoot_Left`
  (params (ActionValue :type Boolean) (ElapsedSeconds :type "Float (double-precision)") (TriggeredSeconds :type "Float (double-precision)") (InputAction :type "InputAction Object Reference" :default "/Game/VRTemplate/Input/Actions/IA_Shoot_Left.IA_Shoot_Left"))
  (:`Started`
    (`KismetSystemLibrary.PrintString` "Hello")
    (if (`|EnumEquality` (`/Game/VRTemplate/Blueprints/GrabComponent.GetHeldByHand` (`self.GrabComponentSnap`)) "Left")
      (`self.FireGun` :!label _label))))

(event `EnhancedInput|/Game/VRTemplate/Input/Actions/IA_Shoot_Right`
  (params (ActionValue :type Boolean) (ElapsedSeconds :type "Float (double-precision)") (TriggeredSeconds :type "Float (double-precision)") (InputAction :type "InputAction Object Reference" :default "/Game/VRTemplate/Input/Actions/IA_Shoot_Right.IA_Shoot_Right"))
  (:`Started`
    (`KismetSystemLibrary.PrintString` "Hello")
    (if (`|EnumEquality` (`/Game/VRTemplate/Blueprints/GrabComponent.GetHeldByHand` (`self.GrabComponentSnap`)) "Right")
      (goto _label))))

(event `self.GrabComponentSnap.OnGrabbed`
  (bind _returnvalue (pcsubsystem `EnhancedInputLocalPlayerSubsystem` (`GameplayStatics.GetPlayerController` 0)))
  ;[1 1 1] Grab Gun
  (`KismetSystemLibrary.PrintString` "Grab ")
  (if (not (`self.IsGrab`))
    (`self.EnableInput` (`GameplayStatics.GetPlayerController` 0))
    (`EnhancedInputSubsystemInterface.AddMappingContext` _returnvalue (select `bool` (`|EnumEquality` (`/Game/VRTemplate/Blueprints/GrabComponent.GetHeldByHand` (`self.GrabComponentSnap`)) "Right") :`false` (`self.IMC_Weapon_Left`) :`true` (`self.IMC_Weapon_Right`)) 1 (struct))
    (set `self.IsGrab` true)
    (`KismetSystemLibrary.PrintString` (`KismetSystemLibrary.GetObjectName` _returnvalue))))

(event `self.GrabComponentSnap.OnDropped`
  ;[1 1 1] Grab Gun
  (`KismetSystemLibrary.PrintString` "Drop ")
  (if (`self.IsGrab`)
    (`self.DisableInput` (`GameplayStatics.GetPlayerController` 0))
    (`EnhancedInputSubsystemInterface.RemoveMappingContext` (pcsubsystem `EnhancedInputLocalPlayerSubsystem` (`GameplayStatics.GetPlayerController` 0)) (select `bool` (`|EnumEquality` (`/Game/VRTemplate/Blueprints/GrabComponent.GetHeldByHand` (`self.GrabComponentSnap`)) "Right") :`false` (`self.IMC_Weapon_Left`) :`true` (`self.IMC_Weapon_Right`)) (struct))
    (set `self.IsGrab` true)))

(fn `Hammer Reload`
  (params (Delta :type "Float (double-precision)"))
  (returns (Reloading :type Boolean))
  (bind (_returnvalue_roll _returnvalue_pitch) (`KismetMathLibrary.BreakRotator` (`SceneComponent.GetSocketRotation` (`self.Hammer`) "None")))
  (bind _returnvalue_roll_2 (`KismetMathLibrary.BreakRotator` (`SceneComponent.GetSocketRotation` (`self.Cylinder`) "None")))
  (if (`self.HammerReloading`)
    (`|ExecutionSequence`
      (:`then_0`
        ;[1 1 1] 해머 장전 동작입니다.
        (set `self.HammerReloading` (< _returnvalue_pitch 50.0))
        (`SceneComponent.K2_SetRelativeRotation` (`self.Hammer`) (`KismetMathLibrary.MakeRotator` 0.0 (+ _returnvalue_pitch (* Delta (`self.HammerRotationSpeed`)))) false false))
      (:`then_1`
        (`SceneComponent.K2_SetRelativeRotation` (`self.Cylinder`) (`KismetMathLibrary.MakeRotator` (+ (* Delta (`self.CylinderRotationSpeed`)) _returnvalue_roll_2)) false false))
      (:`then_2`
        (if (not (== (`self.HammerReloading`) false))
          ;[1 1 1] 총 실린더 값증가
          (set `self.BulletIndex` (mod (+ (`self.BulletIndex`) 1) 6)))
        (return (`self.HammerReloading`))))))

(fn `Load Bullet`
  (returns (NewParam :type "ActorComponent Object Reference"))
  (switch `int` (`self.BulletIndex`)
    (:`Default`
      (set `self.BulletIndex` 0))
    (:`0`
      _)
    (:`1`
      (return (`self.Bullet2`)))
    (:`2`
      (return (`self.Bullet3`)))
    (:`3`
      (return (`self.Bullet4`)))
    (:`4`
      (return (`self.Bullet5`)))
    (:`5`
      (return (`self.Bullet6`))))
  (return (`self.Bullet1`)))

(fn `SettingBulletArray`
  (returns (BulletArray :type "Array of ActorComponent Object Reference"))
  (bind _bullets (`self.Bullets`))
  (`KismetArrayLibrary.Array_Add` _bullets (`self.Bullet1`))
  (`KismetArrayLibrary.Array_Add` _bullets (`self.Bullet2`))
  (`KismetArrayLibrary.Array_Add` _bullets (`self.Bullet3`))
  (`KismetArrayLibrary.Array_Add` _bullets (`self.Bullet4`))
  (`KismetArrayLibrary.Array_Add` _bullets (`self.Bullet5`))
  (`KismetArrayLibrary.Array_Add` _bullets (`self.Bullet6`))
  (return _bullets))

(fn `UserConstructionScript`)