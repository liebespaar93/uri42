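; BP_BulletLife is a grabbable bullet actor that moves along its forward vector at Speed while IsFire is set.
; Movement runs on Tick as a delta-time-scaled location update without sweep.
; GrabComponent events target player 0's input, but hard-coded conditions mean grabbing never enables it and dropping always disables it.
; Nothing in these graphs sets IsFire or handles lifetime or hits.
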(event `self.ReceiveTick`
  (params (DeltaSeconds :type "Float (single-precision)"))
  (if (`self.IsFire`)
    (`self.K2_SetActorLocation` (+ (`self.K2_GetActorLocation`) (* (`self.GetActorForwardVector`) (`self.Speed`) DeltaSeconds)))))

(event `self.GrabComponent.OnGrabbed`
  (if (not true)
    (`self.EnableInput` (`GameplayStatics.GetPlayerController` 0))))

(event `self.GrabComponent.OnDropped`
  (if true
    (`self.DisableInput` (`GameplayStatics.GetPlayerController` 0))))

(fn `UserConstructionScript`)